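; BP_Wildfff is a weapon actor that materializes, spawns a BP_Gun11 child and flies a randomized spline toward AimCoord.
; A reversed timeline animates the material's Amount, then adds light and shadow meshes and sets the spline points.
; A length-scaled timeline moves the mesh and ground shadow, lerping height.
; Box overlaps pause it behind instances further along, and Box or Nose overlaps with Shield-tagged components destroy it.
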(event OnComponentEndOverlap(nose)
  (params (OverlappedComponent :type Primitive%20Component%20Object%20Reference) (OtherActor :type Actor%20Object%20Reference) (OtherComp :type Primitive%20Component%20Object%20Reference) (OtherBodyIndex :type Integer))
  ;[1 1 1 0.2] Comment
  (if (Components|ComponentHasTag OtherComp "Shield")
    ;[1 1 1 0.2] Comment
    (Actor|DestroyActor)))

(event OnComponentBeginOverlap(Box)
  (params (OverlappedComponent :type Primitive%20Component%20Object%20Reference) (OtherActor :type Actor%20Object%20Reference) (OtherComp :type Primitive%20Component%20Object%20Reference) (OtherBodyIndex :type Integer) (bFromSweep :type Boolean) (SweepResult :type Hit%20Result%20Structure%20%28by%20ref%29))
  (Utilities|FlowControl|Sequence
    (:then_0
      ;[1 1 1 0.2] Comment
      (bind _asbp_wildfff (Utilities|Casting|CastToBP_Wildfff OtherActor))
      (if (> (Components|Timeline|GetPlaybackPosition (Variables|BP_Wildfff_C|GetTimeline _asbp_wildfff)) (Components|Timeline|GetPlaybackPosition (Variables|Default|GetTimeline)))
        (Audio|Components|Audio|Stop (Variables|Default|GetTimeline))))
    (:then_2
      ;[1 1 1 0.2] Comment
      (if (Components|ComponentHasTag OtherComp "Shield")
        (Actor|DestroyActor)))))

(event OnComponentEndOverlap(Box)
  (params (OverlappedComponent :type Primitive%20Component%20Object%20Reference) (OtherActor :type Actor%20Object%20Reference) (OtherComp :type Primitive%20Component%20Object%20Reference) (OtherBodyIndex :type Integer))
  (Utilities|FlowControl|Sequence
    (:then_0
      ;[1 1 1 0.2] Comment
      (bind _asbp_wildfff (Utilities|Casting|CastToBP_Wildfff OtherActor))
      (if (> (Components|Timeline|GetPlaybackPosition (Variables|BP_Wildfff_C|GetTimeline _asbp_wildfff)) (Components|Timeline|GetPlaybackPosition (Variables|Default|GetTimeline)))
        (Audio|Components|Audio|Play (Variables|Default|GetTimeline))))
    (:then_1
      ;[1 1 1 0.2] Comment
      (if (Components|ComponentHasTag OtherComp "Shield")
        (Actor|DestroyActor)))))

(event EventBeginPlay
  (bind _returnvalue (Transformation|GetActorLocation))
  (bind _returnvalue_2 (Transformation|GetActorLocation))
  (bind _returnvalue_3 (Math|Random|RandomFloatinRange -1.5e+02 1.5e+02))
  (bind _returnvalue_4 (Math|Random|RandomFloatinRange -1.5e+02 1.5e+02))
  (bind _aimcoord (Variables|Default|GetAimCoord))
  (bind _spline (Variables|Default|GetSpline))
  (bind _staticmesh (Variables|Default|GetStaticMesh))
  (bind _staticmesh_2 (Variables|Default|GetStaticMesh))
  (bind _staticmesh1 (Variables|Default|GetStaticMesh1))
  (bind _square (Variables|Default|Getsquare))
  (bind _spline_2 (Variables|Default|GetSpline))
  (bind _returnvalue_5 (Spline|GetLocationatSplinePoint _spline 2 "World"))
  (bind _returnvalue_6 (Transformation|GetWorldLocation _staticmesh))
  (bind _returnvalue_7 (+ (.x _aimcoord) _returnvalue_3))
  (bind _returnvalue_8 (+ (.y _aimcoord) _returnvalue_4))
  (bind _returnvalue_9 (- _returnvalue _returnvalue_5))
  (bind _returnvalue_10 (/ _returnvalue_9 "2.000000,2.000000,2.000000"))
  ;[1 1 1 0.2] Create wild
  (Components|StaticMesh|SetStaticMesh _staticmesh_2 "/Game/Weapon/Meshes/Wild0.Wild0")
  (Rendering|Material|SetMaterial _staticmesh_2 0 "/Game/Weapon/Materials/MI_Wild0.MI_Wild0")
  (bind _returnvalue_11 (Rendering|Material|CreateDynamicMaterialInstance (Variables|Default|GetStaticMesh) 0 "/Game/Weapon/Materials/MI_Wild0.MI_Wild0" "None" :!class /Script/Engine.PrimitiveComponent))
  (Class|ActorComponent|SetComponentTickInterval (Variables|Default|GetTimeline) 0.04)
  (Components|Timeline|SetPlayRate (Variables|Default|GetTimeline_0) 0.33)
  (bind _amount (Timeline|Timeline_0 ReverseFromEnd)
    (:Update
      (Rendering|Material|SetScalarParameterValue _returnvalue_11 "Amount" _amount :!class /Script/Engine.MaterialInstanceDynamic))
    (:Finished
      (ChildActorComponent|SetChildActorClass (Variables|Default|GetChildActor) "/Game/Weapon/BP_Gun11.BP_Gun11_C")
      (Components|StaticMesh|SetStaticMesh _square "/Game/Weapon/Meshes/square.square")
      (Rendering|Material|SetMaterial _square 0 "/Game/Weapon/Materials/MI_Shadow_Light0.MI_Shadow_Light0")
      (Components|StaticMesh|SetStaticMesh _staticmesh1 "/Game/Weapon/Meshes/Wild0_light.Wild0_light")
      (Rendering|Material|SetMaterial _staticmesh1 0 "/Game/Weapon/Materials/MI_wild0_light.MI_wild0_light")
      (Components|DestroyComponent (Variables|Default|GetTimeline_0))
      (Transformation|SetWorldLocation (Variables|Default|Getsquare) (Math|Vector|MakeVector (.x _returnvalue_6) (.y _returnvalue_6) 0.05) false false)
      ;[1 1 1 0.2] Comment
      (Transformation|SetActorRotation (Math|Rotator|MakeRotator 0.0 0.0 (.yaw (Math|Rotator|FindLookatRotation (Transformation|GetActorLocation) (Math|Vector|MakeVector _returnvalue_7 _returnvalue_8 0.0)))))
      (Spline|SetLocationatSplinePoint _spline 2 (Math|Vector|MakeVector _returnvalue_7 _returnvalue_8 (.z _returnvalue_2)) "World" true)
      (Spline|SetLocationatSplinePoint _spline 1 (Math|Vector|MakeVector (+ (.x _returnvalue_10) (Math|Random|RandomFloatinRange 1e+02 -1e+02)) (+ (.y _returnvalue_10) (Math|Random|RandomFloatinRange 1e+02 -1e+02)) (.z _returnvalue_2)) "World" true)
      ;[1 1 1 0.2] Comment
      (Components|Timeline|SetPlayRate (Variables|Default|GetTimeline) (* (Variables|Default|GetSpeed) (/ 1.0 (Spline|GetSplineLength (Variables|Default|GetSpline)))))
      (Variables|Default|SetHigh (+ (Math|Random|RandomFloatinRange -4e+01 4e+01) (Variables|Default|GetHigh)))
      ;[1 1 1 0.2] Comment
      (bind (_direction _splinerun _high) (Timeline|Timeline PlayFromStart)
        (:Update
          (Transformation|SetWorldLocationAndRotation (Variables|Default|GetStaticMesh) (Math|Vector|MakeVector (.x (Spline|GetLocationatTime _spline_2 _splinerun "World" true)) (.y (Spline|GetLocationatTime _spline_2 _splinerun "World" true)) (Math|Float|Lerp (.z (Transformation|GetActorLocation)) (Variables|Default|GetHigh) _high)) (Math|Rotator|MakeRotator 0.0 0.0 (.yaw (Math|Conversions|RotationFromXVector (Class|SplineComponent|GetDirectionatTime _spline_2 _splinerun "World" true)))) false false)
          (Utilities|IsValid self
            (:Is%20Valid
              (Transformation|SetWorldLocationAndRotation (Variables|Default|Getsquare) (Math|Vector|MakeVector (.x (Spline|GetLocationatTime _spline_2 _splinerun "World" true)) (.y (Spline|GetLocationatTime _spline_2 _splinerun "World" true)) 0.1) (Math|Rotator|MakeRotator 0.0 0.0 (.yaw (Math|Conversions|RotationFromXVector (Class|SplineComponent|GetDirectionatTime _spline_2 _splinerun "World" true)))) false false))))))))

(event Collision|EventActorBeginOverlap
  (params (OtherActor :type Actor%20Object%20Reference)))

(event EventDestroyed)

(fn ConstructionScript)