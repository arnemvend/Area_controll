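; BP_WildFabricfff is a spawner actor that creates BP_Wildfff units aimed at a main tower.
; On BeginPlay it finds BP_Tower actors tagged Main and MainEnemy, keeps the nearer one by horizontal distance as AimCoord, and yaws to face it.
; The Create_Wildff event activates its Niagara effect, spawns a BP_Wildfff slightly above itself with the same rotation, and passes AimCoord to it.
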(event Custom|Create_Wildff
  (bind _returnvalue (Transformation|GetActorLocation))
  ;[1 1 1 0.2] Comment
  (Components|Activation|SetActive (Variables|Default|GetNiagara) true false)
  (bind _returnvalue_2 (Game|SpawnActorfromClass "/Game/Weapon/BP_Wildfff.BP_Wildfff_C" (Math|Transform|MakeTransform (Math|Vector|MakeVector (.x _returnvalue) (.y _returnvalue) (+ (.z _returnvalue) 72.0)) (Transformation|GetActorRotation) "1.000000,1.000000,1.000000") "Undefined" "MultiplyWithRoot" 0 0))
  (Variables|/Game/Weapon/BP_Wildfff.BP_Wildfff_C|SetAimCoord _returnvalue_2 (Variables|Default|GetAimCoord)))

(event EventBeginPlay
  ;[1 1 1 0.2] Comment
  (bind _outactors (Actor|GetAllActorsOfClass "/Game/Buildings/BP_Tower.BP_Tower_C"))
  (for _array_element _outactors
    (if (Actor|ActorHasTag _array_element "Main")
      (Variables|Default|SetAimCoord_Main (Transformation|GetActorLocation _array_element))
      (elif (Actor|ActorHasTag _array_element "MainEnemy")
        (Variables|Default|SetAimCoord_MainEnemy (Transformation|GetActorLocation _array_element)))))
  (if (< (Math|Vector|VectorLengthXY (- (Variables|Default|GetAimCoord_Main) (Transformation|GetActorLocation))) (Math|Vector|VectorLengthXY (- (Variables|Default|GetAimCoord_MainEnemy) (Transformation|GetActorLocation))))
    (Variables|Default|SetAimCoord (Variables|Default|GetAimCoord_Main))
    (else
      (Variables|Default|SetAimCoord (Variables|Default|GetAimCoord_MainEnemy))))
  (Transformation|SetActorRotation (Math|Rotator|MakeRotator 0.0 0.0 (.yaw (Math|Rotator|FindLookatRotation (Transformation|GetActorLocation) (Variables|Default|GetAimCoord))))))

(event Collision|EventActorBeginOverlap
  (params (OtherActor :type Actor%20Object%20Reference)))

(event EventTick
  (params (DeltaSeconds :type Float%20%28single-precision%29)))

(fn ConstructionScript)