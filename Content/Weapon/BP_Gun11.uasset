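; BP_Gun11 is an automatic turret that queues actors entering its capsule through Internal or InternalEnemy tagged components and shoots at the first.
; A Timeline eases rotation toward the target's location, cached at acquisition, then looping timers hold that aim and spawn projectiles with random spread plus Niagara effects.
; When the target becomes invalid or leaves, the timers pause and the next queued target is acquired.
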(event OnComponentBeginOverlap(Capsule)
  (params (OverlappedComponent :type Primitive%20Component%20Object%20Reference) (OtherActor :type Actor%20Object%20Reference) (OtherComp :type Primitive%20Component%20Object%20Reference) (OtherBodyIndex :type Integer) (bFromSweep :type Boolean) (SweepResult :type Hit%20Result%20Structure%20%28by%20ref%29))
  (bind _niagara (Variables|Default|GetNiagara))
  (bind _aims (Variables|Default|GetAims))
  (bind _output (Utilities|Array|Get(acopy) _aims))
  (if (and (Utilities|IsValid OtherActor) (or (Components|ComponentHasTag OtherComp "Internal") (Components|ComponentHasTag OtherComp "InternalEnemy")))
    (Utilities|Array|AddUnique (Variables|Default|GetAims) OtherActor)
    (if (== (Utilities|Array|Length (Variables|Default|GetAims)) 1)
      (Utilities|Time|PauseTimerbyHandle (Variables|Default|GetAimRotTimer))
      (Utilities|Time|PauseTimerbyHandle (Variables|Default|GetFireTimer))
      (if (Utilities|IsValid _output)
        (bind _output_get (Variables|Default|SetAimLoc (Transformation|GetActorLocation _output)))
        ;[1 1 1 0.2] Comment
        (bind _splinerun (Timeline|Timeline PlayFromStart)
          (:Update
            (Transformation|SetActorRotation (Math|Rotator|Lerp(Rotator) (Transformation|GetActorRotation) (Math|Rotator|FindLookatRotation (Transformation|GetActorLocation) _output_get) _splinerun)))
          (:Finished
            (Components|Activation|Activate _niagara false)
            (Effects|Components|ParticleSystem|SetEmitterEnable _niagara "Shooting" true)
            (CallFunction|FireEvent)
            (Utilities|Time|UnpauseTimerbyHandle (Variables|Default|GetAimRotTimer))
            (Utilities|Time|UnpauseTimerbyHandle (Variables|Default|GetFireTimer))
            (bind _returnvalue (Utilities|Time|SetTimerbyEvent (delegate Custom|RotEvent) 0.04 true))
            (Variables|Default|SetAimRotTimer _returnvalue)
            ;[1 1 1 0.2] Comment
            (bind _returnvalue_2 (Utilities|Time|SetTimerbyEvent (delegate Custom|FireEvent) 0.3 true))
            (Variables|Default|SetFireTimer _returnvalue_2)))))))

(event OnComponentEndOverlap(Capsule)
  (params (OverlappedComponent :type Primitive%20Component%20Object%20Reference) (OtherActor :type Actor%20Object%20Reference) (OtherComp :type Primitive%20Component%20Object%20Reference) (OtherBodyIndex :type Integer))
  (if (> (Utilities|Array|Length (Variables|Default|GetAims)) 0)
    (if (== OtherActor (Utilities|Array|Get(acopy) (Variables|Default|GetAims)))
      (Utilities|Time|PauseTimerbyHandle (Variables|Default|GetAimRotTimer))
      (Utilities|Time|PauseTimerbyHandle (Variables|Default|GetFireTimer))
      (Utilities|Array|RemoveItem (Variables|Default|GetAims) OtherActor)
      (if (> (Utilities|Array|Length (Variables|Default|GetAims)) 0)
        (CallFunction|Find))
      (elif (or (Components|ComponentHasTag OtherComp "Internal") (Components|ComponentHasTag OtherComp "InternalEnemy"))
        (Utilities|Array|RemoveItem (Variables|Default|GetAims) OtherActor)))))

(event Custom|RotEvent
  (Transformation|SetActorRotation (Math|Rotator|FindLookatRotation (Transformation|GetActorLocation) (Variables|Default|GetAimLoc)))
  (Utilities|IsValid (Utilities|Array|Get(acopy) (Variables|Default|GetAims))
    (:Is%20Not%20Valid
      (Components|Activation|Deactivate (Variables|Default|GetNiagara))
      (Utilities|Time|PauseTimerbyHandle (Variables|Default|GetAimRotTimer))
      (Utilities|Time|PauseTimerbyHandle (Variables|Default|GetFireTimer))
      (Utilities|Array|RemoveIndex (Variables|Default|GetAims))
      (if (> (Utilities|Array|Length (Variables|Default|GetAims)) 0)
        (CallFunction|Find)))))

(event Custom|FireEvent
  (bind _returnvalue (Transformation|GetActorTransform))
  (bind _accuracy (Variables|Default|GetAccuracy))
  (bind _returnvalue_2 (* _accuracy -1.0))
  ;[1 1 1 0.2] Comment
  (Effects|Components|ParticleSystem|SetVectorParameter (Variables|Default|GetNiagara) "Arrow" (Math|Vector|MakeVector 0.0 0.0 (.yaw (.rotation _returnvalue))))
  (Game|SpawnActorfromClass "/Game/Weapon/prolectile.prolectile_C" (Math|Transform|MakeTransform (.location _returnvalue) (Math|Rotator|MakeRotator (+ (.roll (.rotation _returnvalue)) (Math|Random|RandomFloatinRange _returnvalue_2 _accuracy)) (+ (.pitch (.rotation _returnvalue)) (Math|Random|RandomFloatinRange _returnvalue_2 _accuracy)) (+ (.yaw (.rotation _returnvalue)) (Math|Random|RandomFloatinRange _returnvalue_2 _accuracy))) "1.000000,1.000000,1.000000") "Undefined" "MultiplyWithRoot" 0 0))

(event Custom|find
  (bind _niagara (Variables|Default|GetNiagara))
  (bind _aims (Variables|Default|GetAims))
  (bind _output (Utilities|Array|Get(acopy) _aims))
  (if (Utilities|IsValid _output)
    (bind _output_get (Variables|Default|SetAimLoc (Transformation|GetActorLocation _output)))
    ;[1 1 1 0.2] Comment
    (bind _splinerun (Timeline|Timeline PlayFromStart)
      (:Update
        (Transformation|SetActorRotation (Math|Rotator|Lerp(Rotator) (Transformation|GetActorRotation) (Math|Rotator|FindLookatRotation (Transformation|GetActorLocation) _output_get) _splinerun)))
      (:Finished
        (Components|Activation|Activate _niagara false)
        (Effects|Components|ParticleSystem|SetEmitterEnable _niagara "Shooting" true)
        (CallFunction|FireEvent)
        (Utilities|Time|UnpauseTimerbyHandle (Variables|Default|GetAimRotTimer))
        (Utilities|Time|UnpauseTimerbyHandle (Variables|Default|GetFireTimer))
        (bind _returnvalue (Utilities|Time|SetTimerbyEvent (delegate Custom|RotEvent) 0.04 true))
        (Variables|Default|SetAimRotTimer _returnvalue)
        ;[1 1 1 0.2] Comment
        (bind _returnvalue_2 (Utilities|Time|SetTimerbyEvent (delegate Custom|FireEvent) 0.3 true))
        (Variables|Default|SetFireTimer _returnvalue_2)))))

(event EventBeginPlay
  (Class|ActorComponent|SetComponentTickInterval (Variables|Default|GetTimeline) 0.04)
  (Class|NiagaraComponent|SetAsset (Variables|Default|GetNiagara) "/Game/Weapon/FX/NI_Shoot0.NI_Shoot0" true))

(event Collision|EventActorBeginOverlap
  (params (OtherActor :type Actor%20Object%20Reference)))

(event EventTick
  (params (DeltaSeconds :type Float%20%28single-precision%29)))

(event EventDestroyed
  ;[1 1 1 0.2] Comment
  (Utilities|Time|ClearandInvalidateTimerbyHandle (Variables|Default|GetAimRotTimer))
  (Utilities|Time|ClearandInvalidateTimerbyHandle (Variables|Default|GetFireTimer)))

(fn ConstructionScript)