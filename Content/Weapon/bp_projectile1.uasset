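; Beam-style projectile that follows the nearest BP_Gun11 for a timed burst, then destroys itself.
; On BeginPlay a throttled Timeline starts, snapping the actor to the gun, line tracing and updating the Niagara beam endpoints on each update.
; The hit component's tag selects a shield, object or ground effect, spawned as BP_Boom.
; Only Internal and InternalEnemy hits apply damage, repeatedly while the trace stays on them.
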(event EventBeginPlay
  (bind _returnvalue (Transformation|GetActorLocation))
  (bind _timeline (Variables|Default|GetTimeline))
  (bind _outactors (Actor|GetAllActorsOfClass "/Game/Weapon/BP_Gun11.BP_Gun11_C"))
  (Variables|Default|SetGun_ref (.ReturnValue (Actor|FindNearestActor (Transformation|GetActorLocation) _outactors)))
  (Class|ActorComponent|SetComponentTickInterval _timeline 0.04)
  (Components|Timeline|SetPlayRate _timeline 0.5)
  (Timeline|Timeline PlayFromStart
    (:Update
      (Transformation|SetActorTransform (Math|Transform|MakeTransform (.location (Transformation|GetActorTransform (Variables|Default|GetGun_ref))) (Math|Rotator|MakeRotator (.roll (.rotation (Transformation|GetActorTransform (Variables|Default|GetGun_ref)))) (.pitch (.rotation (Transformation|GetActorTransform (Variables|Default|GetGun_ref)))) (.yaw (.rotation (Transformation|GetActorTransform (Variables|Default|GetGun_ref))))) "1.000000,1.000000,1.000000"))
      (Effects|Components|ParticleSystem|SetVectorParameter (Variables|Default|GetNI_Shoot1) "Start" _returnvalue)
      (bind _outhit (Collision|LineTraceByChannel _returnvalue (Math|Vector|MakeVector 0.0 0.0 (.z (* (Transformation|GetActorForwardVector) 1e+03))) "TraceTypeQuery1" false 0 "ForOneFrame"))
      (Effects|Components|ParticleSystem|SetVectorParameter (Variables|Default|GetNI_Shoot1) "End" (.Location (Collision|BreakHitResult _outhit)))
      (if (Components|ComponentHasTag (.HitComponent (Collision|BreakHitResult _outhit)) "Shield")
        (bind _returnvalue_2 (Game|SpawnActorfromClass "/Game/Weapon/FX/BP_Boom.BP_Boom_C" (Math|Transform|MakeTransform (.Location (Collision|BreakHitResult _outhit)) (Math|Rotator|FindLookatRotation (Transformation|GetActorLocation (.HitActor (Collision|BreakHitResult _outhit))) (.Location (Collision|BreakHitResult _outhit))) "1.000000,1.000000,1.000000") "Undefined" "MultiplyWithRoot" 0 0))
        (Class|NiagaraComponent|SetAsset (Variables|/Game/Weapon/FX/BP_Boom.BP_Boom_C|GetNiagara _returnvalue_2) "/Game/Weapon/FX/NI_Boom0_sh.NI_Boom0_sh" false)
        (Variables|/Game/Weapon/FX/BP_Boom.BP_Boom_C|SetDuration _returnvalue_2 (Variables|Default|GetDuration))
        (Default|BoomEvent _returnvalue_2)
        (elif (or (Components|ComponentHasTag (.HitComponent (Collision|BreakHitResult _outhit)) "Internal") (Components|ComponentHasTag (.HitComponent (Collision|BreakHitResult _outhit)) "InternalEnemy"))
          (if (Utilities|IsValid (.HitActor (Collision|BreakHitResult _outhit)))
            (Game|Damage|ApplyDamage (.HitActor (Collision|BreakHitResult _outhit)) (Variables|Default|GetDamage) 0 0)
            (bind _returnvalue_3 (Game|SpawnActorfromClass "/Game/Weapon/FX/BP_Boom.BP_Boom_C" (Math|Transform|MakeTransform (.Location (Collision|BreakHitResult _outhit)) "0, 0, 0" "1.000000,1.000000,1.000000") "Undefined" "MultiplyWithRoot" 0 0))
            (Class|NiagaraComponent|SetAsset (Variables|/Game/Weapon/FX/BP_Boom.BP_Boom_C|GetNiagara _returnvalue_3) "/Game/Weapon/FX/NI_Boom0_obj.NI_Boom0_obj" false)
            (Variables|/Game/Weapon/FX/BP_Boom.BP_Boom_C|SetDuration _returnvalue_3 (Variables|Default|GetDuration))
            (Default|BoomEvent _returnvalue_3))
          (elif (Components|ComponentHasTag (.HitComponent (Collision|BreakHitResult _outhit)) "Ground")
            (bind _returnvalue_4 (Game|SpawnActorfromClass "/Game/Weapon/FX/BP_Boom.BP_Boom_C" (Math|Transform|MakeTransform (.Location (Collision|BreakHitResult _outhit)) "0, 0, 0" "1.000000,1.000000,1.000000") "Undefined" "MultiplyWithRoot" 0 0))
            (Class|NiagaraComponent|SetAsset (Variables|/Game/Weapon/FX/BP_Boom.BP_Boom_C|GetNiagara _returnvalue_4) "/Game/Weapon/FX/NI_Boom0_gr.NI_Boom0_gr" false)
            (Variables|/Game/Weapon/FX/BP_Boom.BP_Boom_C|SetDuration _returnvalue_4 (Variables|Default|GetDuration))
            (Default|BoomEvent _returnvalue_4)))))
    (:Finished
      (Actor|DestroyActor))))

(event Collision|EventActorBeginOverlap
  (params (OtherActor :type Actor%20Object%20Reference)))

(event EventTick
  (params (DeltaSeconds :type Float%20%28single-precision%29)))

(fn ConstructionScript)