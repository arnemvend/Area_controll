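; Player controller for the area-control game, turning touch, pinch and mouse wheel input into camera movement and building placement.
; On begin play it caches the ground, camera and main tower, and forces lowest graphics settings.
; Touches projected to world space pan the camera, or each tick drag an active build creator while feeding screen position to the camera.
; Releasing a ready creator spawns a construction in the main tower's color.
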(event Custom|PressReset
  ;[1 1 1 0.2] Camera control
  (Utilities|FlowControl|DoOnce false) ; enters at Reset
)

(event EventBeginPlay
  (Utilities|FlowControl|Sequence
    (:then_0
      ;[1 1 1 0.2] References
      (bind _returnvalue (Actor|GetActorOfClass "/Game/Map/BP_GroundActor.BP_GroundActor_C"))
      (Variables|Default|SetGroundActor_ref _returnvalue)
      (bind _returnvalue_2 (Actor|GetActorOfClass "/Game/PCamera/BP_PlayerCamera.BP_PlayerCamera_C"))
      (Variables|Default|SetPlayerCamera_ref _returnvalue_2)
      (bind _outactors (Actor|GetAllActorsOfClass "/Script/Engine.Actor"))
      (bind _output_get (Variables|Default|SetOut%20Actors _outactors))
      (Utilities|Array|RemoveItem _output_get (Variables|Default|GetGroundActor_ref))
      (bind _outactors_2 (Actor|GetAllActorsOfClass "/Game/Buildings/BP_Tower.BP_Tower_C"))
      (for _array_element _outactors_2
        (if (Actor|ActorHasTag _array_element "Main")
          (Variables|Default|SetMainTower _array_element))))
    (:then_1
      (bind _returnvalue_3 (Settings|GetGameUserSettings))
      (Class|GameUserSettings|SetVSyncEnabled _returnvalue_3 false)
      (Class|GameUserSettings|SetViewDistanceQuality _returnvalue_3)
      (Class|GameUserSettings|SetAntiAliasingQuality _returnvalue_3)
      (Class|GameUserSettings|SetPostProcessingQuality _returnvalue_3)
      (Class|GameUserSettings|SetShadowQuality _returnvalue_3)
      (Class|GameUserSettings|SetGlobalIlluminationQuality _returnvalue_3)
      (Class|GameUserSettings|SetReflectionQuality _returnvalue_3)
      (Class|GameUserSettings|SetTextureQuality _returnvalue_3)
      (Class|GameUserSettings|SetVisualEffectQuality _returnvalue_3)
      (Class|GameUserSettings|SetShadingQuality _returnvalue_3)
      (Class|GameUserSettings|SetFoliageQuality _returnvalue_3)
      (Class|GameUserSettings|ApplySettings _returnvalue_3 true)
      (Class|GameUserSettings|SaveSettings _returnvalue_3))))

(event EventTick
  (params (DeltaSeconds :type Float%20%28single-precision%29))
  (if (Variables|Default|GetCreatorIsHere)
    (Utilities|IsValid (Variables|Default|GetBuildCreator_ref)
      (:Is%20Valid
        ;[1 1 1 0.2] Build Creator control
        (Class|BuildCreator|MovingFunc (Variables|Default|GetBuildCreator_ref) (Class|MyBlueprintFunctionLibrary|TouchtoWorld (.x (stale Input|TouchEvents|InputTouch Location)) (.y (stale Input|TouchEvents|InputTouch Location)) (Variables|Default|GetOut%20Actors) (Game|GetPlayerController 0) self) 1.0)
        (Class|PlayerCamera|CameraMove (Variables|Default|GetPlayerCamera_ref) (Math|Vector2D|MakeVector2D (.x (stale Input|TouchEvents|InputTouch Location)) (.y (stale Input|TouchEvents|InputTouch Location))) (Viewport|GetViewportSize))))))

(event Input|AxisEvents|InputAxisPinch
  (params (AxisValue :type Float%20%28single-precision%29))
  ;[1 1 1 0.2] Camera zoom control
  (Utilities|IsValid (Variables|Default|GetBuildCreator_ref)
    (:Is%20Not%20Valid
      (if (Variables|Default|GetIsPinch)
        (Class|PlayerCamera|CameraZoom (Variables|Default|GetPlayerCamera_ref) AxisValue (Variables|Default|GetInitDistance))
        (Variables|Default|SetInitDistance AxisValue)))))

(event Input|MouseEvents|MouseWheelAxis
  (params (AxisValue :type Float%20%28single-precision%29))
  (Class|PlayerCamera|CameraZoom (Variables|Default|GetPlayerCamera_ref) AxisValue 0.0))

(event Input|KeyboardEvents|GesturePinch
  (params (Key :type Key%20Structure :default "None"))
  ;[1 1 1 0.2] Camera zoom control
  (:Pressed
    (Utilities|IsValid (Variables|Default|GetBuildCreator_ref)
      (:Is%20Not%20Valid
        (Variables|Default|SetIsPinch true)
        (Utilities|FlowControl|DoOnce false :!label _label
          (:Completed
            (Variables|Default|SetInitDistance 1.0))))))
  (:Released
    (Utilities|FlowControl|Delay 0.2)
    (Variables|Default|SetIsPinch false)
    (goto _label Reset)))

(event Input|TouchEvents|InputTouch
  (params (Location :type Vector) (FingerIndex :type ETouchIndex%20Enum))
  (bind _returnvalue (Game|GetPlayerController 0))
  (bind _self self)
  (bind _buildcreator_ref (Variables|Default|GetBuildCreator_ref))
  (bind _out_actors (Variables|Default|GetOut%20Actors))
  (bind _playercamera_ref (Variables|Default|GetPlayerCamera_ref))
  (bind _position (Class|MyBlueprintFunctionLibrary|TouchtoWorld (.x Location) (.y Location) _out_actors _returnvalue _self))
  (:Pressed
    (Utilities|IsValid (Variables|Default|GetBuildCreator_ref)
      (:Is%20Not%20Valid
        (if (not (Variables|Default|GetIsPinch))
          ;[1 1 1 0.2] Camera control
          (Utilities|FlowControl|DoOnce false
            (:Completed
              (Class|PlayerCamera|StartTouchMove _playercamera_ref _position)))))))
  (:Released
    (CallFunction|PressReset)
    ;[1 1 1 0.2] Destroy Build Crearor
    (Utilities|IsValid _buildcreator_ref
      (:Is%20Valid
        (if (Variables|/Script/Area_controll.BuildCreator|GetIsReady _buildcreator_ref)
          (bind _returnvalue_2 (Game|SpawnActorfromClass "/Game/Buildings/BP_Construction.BP_Construction_C" (Transformation|GetActorTransform _buildcreator_ref) "Undefined" "MultiplyWithRoot" 0 0))
          (Variables|/Game/Buildings/BP_Construction.BP_Construction_C|SetColor _returnvalue_2 (Variables|/Script/Area_controll.Tower|GetYourColorGround (Variables|Default|GetMainTower)))
          (Default|ColorEvent _returnvalue_2))
        (Class|BuildCreator|DestroyerFunc (Variables|Default|GetBuildCreator_ref))
        (Utilities|Array|Clear (Variables|Default|GetOut%20Actors))
        (Variables|Default|SetCreatorIsHere false))))
  (:Moved
    (Utilities|IsValid (Variables|Default|GetBuildCreator_ref)
      (:Is%20Not%20Valid
        (if (not (Variables|Default|GetIsPinch))
          (Class|PlayerCamera|TouchMove _playercamera_ref _position))))))

(fn ConstructionScript)