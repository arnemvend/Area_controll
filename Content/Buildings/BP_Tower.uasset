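; BP_Tower is a tower building that responds to touch, takes damage and explodes when destroyed.
; BeginPlay binds touch to Touch and hands itself to its TowerWidget menu.
; Damage lowers Health only while both shield meshes are hidden, updates the dynamic material's Damage parameter with the health ratio, and calls TowerDestroy at zero.
; On Destroyed, it spawns a BP_Boom configured with the tower's Niagara explosion.
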(event Custom|SetDamageEvent
  (Rendering|Material|SetScalarParameterValue (Variables|Default|GetDTowMaterial) "Damage" (/ (Variables|Default|GetHealth) (Variables|Default|GetMaxHealth)) :!class /Script/Engine.MaterialInstanceDynamic)
  (if (not (> (Variables|Default|GetHealth) 0.0))
    (Class|Tower|TowerDestroy)))

(event Custom|OnInputTouchBegin_Event
  (params (FingerIndex :type ETouchIndex%20Enum :default "Touch1") (TouchedActor :type Actor%20Object%20Reference))
  ;[1 1 1 0.2] Touch event
  (Class|Tower|Touch))

(event EventBeginPlay
  ;[1 1 1 0.2] Touch event
  (EventDispatchers|BindEventtoOnInputTouchBegin (delegate Custom|OnInputTouchBegin_Event))
  ;[1 1 1 0.2] Binding TowerWidget
  (bind _asbp_tower_menu (Utilities|Casting|CastToBP_TowerMenu (UserInterface|GetUserWidgetObject (Variables|Default|GetTowerWidget))))
  (Variables|/Game/HUD/BP_TowerMenu.BP_TowerMenu_C|SetMyTower_ref _asbp_tower_menu self))

(event Collision|EventActorBeginOverlap
  (params (OtherActor :type Actor%20Object%20Reference)))

(event EventDestroyed
  (bind _returnvalue (Game|SpawnActorfromClass "/Game/Weapon/FX/BP_Boom.BP_Boom_C" (Math|Transform|MakeTransform (Transformation|GetActorLocation) "0, 0, 0" "1.000000,1.000000,1.000000") "Undefined" "MultiplyWithRoot" 0 0))
  (Class|NiagaraComponent|SetAsset (Variables|/Game/Weapon/FX/BP_Boom.BP_Boom_C|GetNiagara _returnvalue) "/Game/Buildings/FX/NI_BoomTower.NI_BoomTower" false)
  (Variables|/Game/Weapon/FX/BP_Boom.BP_Boom_C|SetDuration _returnvalue 2.0)
  (Default|BoomEvent _returnvalue))

(event Game|Damage|EventAnyDamage
  (params (Damage :type Float%20%28single-precision%29) (DamageType :type Damage%20Type%20Object%20Reference) (InstigatedBy :type Controller%20Object%20Reference) (DamageCauser :type Actor%20Object%20Reference))
  (if (Math|Boolean|ANDBoolean (> (Variables|Default|GetHealth) 0.0) (not (Rendering|IsVisible (Variables|Default|GetSphereShieldMesh))) (not (Rendering|IsVisible (Variables|Default|GetPartShieldMesh))))
    (Variables|Default|SetHealth (- (Variables|Default|GetHealth) Damage))
    (Rendering|Material|SetScalarParameterValue (Variables|Default|GetDTowMaterial) "Damage" (/ (Variables|Default|GetHealth) (Variables|Default|GetMaxHealth)) :!class /Script/Engine.MaterialInstanceDynamic)
    (if (not (> (Variables|Default|GetHealth) 0.0))
      (Class|Tower|TowerDestroy))))

(fn ConstructionScript)