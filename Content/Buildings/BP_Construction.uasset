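; Building construction site that gains health over time and replaces itself with a BP_Tower once construction completes.
; Looping timers rotate the builder mesh and raise both Health and build progress (HealthP) each second.
; Damage lowers only Health, destroying the site at zero; otherwise the finished tower inherits the Health/Max fraction.
; ColorEvent tints both meshes through dynamic material instances using the Color variable.
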(event Custom|RotEvent
  (Transformation|AddWorldRotation (Variables|Default|GetStaticMesh) "0.000000,0.500000,0.000000" false false))

(event Custom|PlusHealth
  (Variables|Default|SetHealth (+ (Variables|Default|GetHealth) 2.0))
  (bind _output_get (Variables|Default|SetHealth_P (+ (Variables|Default|GetHealth_P) 2.0)))
  (if (>= _output_get (Variables|Default|GetMax))
    (bind _returnvalue (Game|SpawnActorfromClass "/Game/Buildings/BP_Tower.BP_Tower_C" (Math|Transform|MakeTransform (Transformation|GetActorLocation) "0, 0, 0" "1.000000,1.000000,1.000000") "Undefined" "MultiplyWithRoot" 0 0))
    (Variables|/Script/Area_controll.Tower|SetHealth _returnvalue (* (Variables|/Script/Area_controll.Tower|GetMaxHealth _returnvalue) (/ (Variables|Default|GetHealth) (Variables|Default|GetMax))))
    (Default|SetDamageEvent _returnvalue)
    (Actor|DestroyActor)))

(event Custom|ColorEvent
  (bind _returnvalue (Rendering|Material|CreateDynamicMaterialInstance (Variables|Default|GetStaticMesh1) 0 "/Game/Buildings/Materials/MI_Construct.MI_Construct" "None" :!class /Script/Engine.PrimitiveComponent))
  (Rendering|Material|SetVectorParameterValue _returnvalue "Color" (Math|Conversions|ToLinearColor(Color) (Variables|Default|GetColor)) :!class /Script/Engine.MaterialInstanceDynamic)
  (bind _returnvalue_2 (Rendering|Material|CreateDynamicMaterialInstance (Variables|Default|GetStaticMesh) 0 "/Game/Buildings/Materials/MI_Builder.MI_Builder" "None" :!class /Script/Engine.PrimitiveComponent))
  (Rendering|Material|SetVectorParameterValue _returnvalue_2 "Color" (Math|Conversions|ToLinearColor(Color) (Variables|Default|GetColor)) :!class /Script/Engine.MaterialInstanceDynamic))

(event EventBeginPlay
  (bind _returnvalue (Utilities|Time|SetTimerbyEvent (delegate Custom|RotEvent) 0.04 true))
  (Variables|Default|SetNewVar _returnvalue)
  (bind _returnvalue_2 (Utilities|Time|SetTimerbyEvent (delegate Custom|PlusHealth) 1.0 true))
  (Variables|Default|SetNewVar_0 _returnvalue_2))

(event Collision|EventActorBeginOverlap
  (params (OtherActor :type Actor%20Object%20Reference)))

(event EventTick
  (params (DeltaSeconds :type Float%20%28single-precision%29)))

(event Game|Damage|EventAnyDamage
  (params (Damage :type Float%20%28single-precision%29) (DamageType :type Damage%20Type%20Object%20Reference) (InstigatedBy :type Controller%20Object%20Reference) (DamageCauser :type Actor%20Object%20Reference))
  (Variables|Default|SetHealth (- (Variables|Default|GetHealth) Damage))
  (if (not (> (Variables|Default|GetHealth) 0.0))
    (Actor|DestroyActor)))

(event EventDestroyed
  (Utilities|Time|ClearandInvalidateTimerbyHandle (Variables|Default|GetNewVar_0))
  (Utilities|Time|ClearandInvalidateTimerbyHandle (Variables|Default|GetNewVar)))

(fn ConstructionScript)